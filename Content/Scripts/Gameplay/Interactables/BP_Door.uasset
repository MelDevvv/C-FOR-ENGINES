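; Interactable door Blueprint that slides its Cube mesh open when interacted with.
; Interact prints who used the door, then calls OpenDoor or CloseDoor based on IsOpen.
; OpenDoor plays a timeline that lerps the cube from its BeginPlay position by DoorOpenOffset, setting IsOpen from the direction on finish.
; CloseDoor only stops the timeline, so the door never moves back.
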(event Custom|OpenDoor
  (bind _doorclosed (Variables|Default|GetDoorClosed))
  (bind (_direction _alpha) (Timeline|T_Door Play)
    (:Update
      (Transformation|SetWorldLocation (Variables|Default|GetCube) (Math|Vector|Lerp(Vector) _doorclosed (+ _doorclosed (Variables|Default|GetDoorOpenOffset)) _alpha) false false))
    (:Finished
      (Variables|Default|SetbIsOpen (Utilities|Select :Index _direction :Forward true :Backward false)))))

(event Custom|CloseDoor
  (bind _doorclosed (Variables|Default|GetDoorClosed))
  (bind (_direction _alpha) (Timeline|T_Door Stop)
    (:Update
      (Transformation|SetWorldLocation (Variables|Default|GetCube) (Math|Vector|Lerp(Vector) _doorclosed (+ _doorclosed (Variables|Default|GetDoorOpenOffset)) _alpha) false false))
    (:Finished
      (Variables|Default|SetbIsOpen (Utilities|Select :Index _direction :Forward true :Backward false)))))

(event EventBeginPlay
  (Variables|Default|SetDoorClosed (Transformation|GetWorldLocation (Variables|Default|GetCube))))

(event EventInteract
  (params (InteractorPawn :type Pawn%20Object%20Reference))
  (Utilities|IsValid InteractorPawn
    (:Is%20Valid
      (Development|PrintString (Utilities|String|Append (Utilities|GetDisplayName InteractorPawn) " Opened Door")))
    (:Is%20Not%20Valid
      (Development|PrintString "Door Open")))
  (if (Variables|Default|GetbIsOpen)
    (CallFunction|CloseDoor)
    (else
      (CallFunction|OpenDoor))))

(fn ConstructionScript)