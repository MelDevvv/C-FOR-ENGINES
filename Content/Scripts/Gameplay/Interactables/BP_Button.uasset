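; BP_Button is a pressure-style button that triggers linked actors when a pawn steps into its sphere trigger.
; The first pawn to overlap sends InteractMessage to every entry in LinkedActors, turns the cylinder to the good material and sets IsPressed, blocking repeat triggers.
; When no pawns remain overlapping, it restores the danger material and clears IsPressed without notifying the linked actors.
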(event OnComponentBeginOverlap(Sphere)
  (params (OverlappedComponent :type Primitive%20Component%20Object%20Reference) (OtherActor :type Actor%20Object%20Reference) (OtherComp :type Primitive%20Component%20Object%20Reference) (OtherBodyIndex :type Integer) (bFromSweep :type Boolean) (SweepResult :type Hit%20Result%20Structure%20%28by%20ref%29))
  ;[0.9043 0.05026 0 0.5] Button Overlap Events
  (bind _aspawn (Utilities|Casting|CastToPawn OtherActor))
  (if (not (Variables|Default|GetbIsPressed))
    (for _array_element (Variables|Default|GetLinkedActors)
      (Class|BPIInteract|Interact(Message) _array_element _aspawn))
    (CallFunction|ButtonTriggered)))

(event OnComponentEndOverlap(Sphere)
  (params (OverlappedComponent :type Primitive%20Component%20Object%20Reference) (OtherActor :type Actor%20Object%20Reference) (OtherComp :type Primitive%20Component%20Object%20Reference) (OtherBodyIndex :type Integer))
  ;[0.9043 0.05026 0 0.5] Button Overlap Events
  (if (Utilities|Array|IsEmpty (Collision|GetOverlappingActors (Variables|Default|GetSphere) "/Script/Engine.Pawn" :!class /Script/Engine.PrimitiveComponent))
    (CallFunction|ResetButton)))

(event Custom|ButtonTriggered
  ;[1 0.751 0 0.5] Button Material Events
  (Rendering|Material|SetMaterial (Variables|Default|GetCylinder) 0 "/Game/Assets/Materials/Grids/MI_Grid_Good.MI_Grid_Good")
  (Variables|Default|SetbIsPressed true))

(event Custom|ResetButton
  ;[1 0.751 0 0.5] Button Material Events
  (Rendering|Material|SetMaterial (Variables|Default|GetCylinder) 0 "/Game/Assets/Materials/Grids/MI_Grid_Danger.MI_Grid_Danger")
  (Variables|Default|SetbIsPressed false))

(fn ConstructionScript)