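; BP_TankController is the controller that turns player input into commands for the tank pawn it controls.
; On possess, it checks that the pawn is valid and adds the IMC_Tank mapping context to the Enhanced Input local player subsystem.
; Forward, turn and fire actions pass their values to the controlled pawn as move, turn and primary action interface messages, so no cast to a tank class is needed.
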(event Input|EnhancedActionEvents|EnhancedInputActionIA_Forward
  (params (ActionValue :type Float%20%28double-precision%29) (ElapsedSeconds :type Float%20%28double-precision%29) (TriggeredSeconds :type Float%20%28double-precision%29) (InputAction :type Input%20Action%20Object%20Reference :default "/Game/Assets/Input/IA_Forward.IA_Forward"))
  ;[0 0.6464 0.7826 0.8435] Input Actions
  (Class|Inputable|IMove(Message) (Pawn|GetControlledPawn) ActionValue))

(event Input|EnhancedActionEvents|EnhancedInputActionIA_Turn
  (params (ActionValue :type Float%20%28double-precision%29) (ElapsedSeconds :type Float%20%28double-precision%29) (TriggeredSeconds :type Float%20%28double-precision%29) (InputAction :type Input%20Action%20Object%20Reference :default "/Game/Assets/Input/IA_Turn.IA_Turn"))
  ;[0 0.6464 0.7826 0.8435] Input Actions
  (Class|Inputable|ITurn(Message) (Pawn|GetControlledPawn) ActionValue))

(event Input|EnhancedActionEvents|EnhancedInputActionIA_Fire
  (params (ActionValue :type Boolean) (ElapsedSeconds :type Float%20%28double-precision%29) (TriggeredSeconds :type Float%20%28double-precision%29) (InputAction :type Input%20Action%20Object%20Reference :default "/Game/Assets/Input/IA_Fire.IA_Fire"))
  ;[0 0.6464 0.7826 0.8435] Input Actions
  (Class|Inputable|IPrimaryAction(Message) (Pawn|GetControlledPawn) ActionValue))

(event EventPossess
  (params (PossessedPawn :type Pawn%20Object%20Reference))
  ;[0.09237 0.8348 0 0.5] On Possess
  (Utilities|IsValid PossessedPawn
    (:Is%20Valid
      (Input|AddMappingContext (PlayerController|LocalPlayerSubsystems|GetEnhancedInputLocalPlayerSubsystem) "/Game/Assets/Input/IMC_Tank.IMC_Tank" 0 "(bIgnoreAllPressedKeysUntilRelease=True,bForceImmediately=False,bNotifyUserSettings=False)"))))

(fn ConstructionScript)